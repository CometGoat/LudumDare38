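; BP_BarrierBot is a bot that links with nearby barrier bots to form beam barriers that destroy nanobots.
; Sphere overlaps add or remove other barrier bots in an array, with a parallel array holding a P_Barrier beam emitter per link.
; Each Tick line-traces to every linked bot and destroys any BP_NanoBot the trace hits.
; If Moving is set, BeginPlay gives it constant local forward velocity through ProjectileMovement.
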(event `self.ReceiveBeginPlay`
  (if (`self.Moving`)
    (`ProjectileMovementComponent.SetVelocityInLocalSpace` (`self.ProjectileMovement`) (300.0 0.0 0.0))))

(event `self.ReceiveTick`
  (params (DeltaSeconds :type "Float (single-precision)"))
  (for (_array_element _array_index) (`self.BarrierArray`)
    (bind _outhit (`KismetSystemLibrary.LineTraceSingle` (`self.K2_GetActorLocation`) (`self.K2_GetActorLocation` _array_element) "TraceTypeQuery1"))
    (bind _asbp_nano_bot (cast `/Game/Characters/CharactersBlueprints/BP_NanoBot` (`.HitActor` (`GameplayStatics.BreakHitResult` _outhit))))
    (`self.K2_DestroyActor` _asbp_nano_bot)))

(event `self.Sphere.OnComponentBeginOverlap`
  (params (OverlappedComponent :type "PrimitiveComponent Object Reference") (OtherActor :type "Actor Object Reference") (OtherComp :type "PrimitiveComponent Object Reference") (OtherBodyIndex :type Integer) (bFromSweep :type Boolean) (SweepResult :type "HitResult Structure (by ref)"))
  (bind _asbp_barrier_bot (cast `/Game/Characters/CharactersBlueprints/BP_BarrierBot` OtherActor))
  (if (not (`KismetArrayLibrary.Array_Contains` (`self.BarrierArray`) _asbp_barrier_bot))
    (bind _returnvalue (`KismetArrayLibrary.Array_AddUnique` (`self.BarrierArray`) _asbp_barrier_bot))
    (bind _returnvalue_2 (`GameplayStatics.SpawnEmitterAttached` "/Game/Effects/Particles/P_Barrier.P_Barrier" (`self.Cube`)))
    (set `ParticleSystemComponent.InstanceParameters` (`|MakeArray` (make `ParticleSysParam` "BeamSource" "PSPT_Actor" 0.0 0.0 (0.0 0.0 0.0) (0.0 0.0 0.0) (struct) self) (make `ParticleSysParam` "BeamTarget" "PSPT_Actor" 0.0 0.0 (0.0 0.0 0.0) (0.0 0.0 0.0) (struct) _asbp_barrier_bot)) _returnvalue_2)
    (`KismetArrayLibrary.Array_Set` (`self.ParticleArray`) _returnvalue _returnvalue_2 true)))

(event `self.Sphere.OnComponentEndOverlap`
  (params (OverlappedComponent :type "PrimitiveComponent Object Reference") (OtherActor :type "Actor Object Reference") (OtherComp :type "PrimitiveComponent Object Reference") (OtherBodyIndex :type Integer))
  (bind _barrierarray (`self.BarrierArray`))
  (bind _particlearray (`self.ParticleArray`))
  (bind _asbp_barrier_bot (cast `/Game/Characters/CharactersBlueprints/BP_BarrierBot` OtherActor))
  (if (`KismetArrayLibrary.Array_Contains` _barrierarray _asbp_barrier_bot)
    (bind _returnvalue (`KismetArrayLibrary.Array_Find` _barrierarray _asbp_barrier_bot))
    (`ActorComponent.K2_DestroyComponent` (`KismetArrayLibrary.Array_Get` _particlearray _returnvalue))
    (`KismetArrayLibrary.Array_Remove` _particlearray _returnvalue)
    (`KismetArrayLibrary.Array_RemoveItem` _barrierarray _asbp_barrier_bot)))

(fn `UserConstructionScript`)