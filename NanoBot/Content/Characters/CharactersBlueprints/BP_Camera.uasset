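; BP_Camera is the player's follow camera for BP_NanoBot, with a rising shot for death.
; After a short delay at BeginPlay it becomes player 0's view target and assigns itself to every BP_NanoBot.
; Tick keeps it at an offset from its referenced bot until PlayerDead is set.
; The DeathCam event moves it steadily upward, re-calling itself through a zero-length Delay as an endless per-frame loop.
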(event `self.ReceiveBeginPlay`
  (`KismetSystemLibrary.Delay` 0.2)
  (`PlayerController.SetViewTargetWithBlend` (`GameplayStatics.GetPlayerController` 0) self 0.0 "VTBlend_Linear" 0.0 false)
  (bind _outactors (`GameplayStatics.GetAllActorsOfClass` "/Game/Characters/CharactersBlueprints/BP_NanoBot.BP_NanoBot_C"))
  (for _array_element _outactors
    (set `/Game/Characters/CharactersBlueprints/BP_NanoBot.BP_Camera` self _array_element)))

(event `self.ReceiveTick`
  (params (DeltaSeconds :type "Float (single-precision)"))
  (bind _bp_nanobot (`self.BP_NanoBot`))
  (if (not (`self.PlayerDead`))
    (`/Engine/EditorBlueprintResources/StandardMacros.IsValid` _bp_nanobot
      (:`Is Valid`
        (`self.K2_SetActorLocation` (+ (`self.K2_GetActorLocation` _bp_nanobot) (`self.Offset`)))))))

(event `DeathCam`
  (`self.K2_SetActorLocation` (`KismetMathLibrary.MakeVector` (.x (`self.K2_GetActorLocation`)) (.y (`self.K2_GetActorLocation`)) (+ (.z (`self.K2_GetActorLocation`)) (* (`GameplayStatics.GetWorldDeltaSeconds`) 1000.0))))
  (`KismetSystemLibrary.Delay` 0.0)
  (`self.DeathCam`))

(fn `UserConstructionScript`)