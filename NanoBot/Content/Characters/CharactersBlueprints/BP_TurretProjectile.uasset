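; Turret projectile actor that destroys any BP_NanoBot it strikes.
; Its Sphere's begin-overlap and hit events run duplicate cast chains that ignore BP_BarrierBot and BP_TurretBot.
; Contact with any other actor destroys the projectile, taking the other actor with it only if that is a NanoBot.
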(event `self.Sphere.OnComponentBeginOverlap`
  (params (OverlappedComponent :type "PrimitiveComponent Object Reference") (OtherActor :type "Actor Object Reference") (OtherComp :type "PrimitiveComponent Object Reference") (OtherBodyIndex :type Integer) (bFromSweep :type Boolean) (SweepResult :type "HitResult Structure (by ref)"))
  (cast `/Game/Characters/CharactersBlueprints/BP_BarrierBot` OtherActor
    (:`CastFailed`
      (cast `/Game/Characters/CharactersBlueprints/BP_TurretBot` OtherActor
        (:`CastFailed`
          (bind _asbp_nano_bot (cast `/Game/Characters/CharactersBlueprints/BP_NanoBot` OtherActor)
            (:`then`
              (`self.K2_DestroyActor` _asbp_nano_bot))
            (:`CastFailed`
              _))
          (`self.K2_DestroyActor`))))))

(event `self.Sphere.OnComponentHit`
  (params (HitComponent :type "PrimitiveComponent Object Reference") (OtherActor :type "Actor Object Reference") (OtherComp :type "PrimitiveComponent Object Reference") (NormalImpulse :type "Vector Structure") (Hit :type "HitResult Structure (by ref)"))
  (cast `/Game/Characters/CharactersBlueprints/BP_BarrierBot` OtherActor
    (:`CastFailed`
      (cast `/Game/Characters/CharactersBlueprints/BP_TurretBot` OtherActor
        (:`CastFailed`
          (bind _asbp_nano_bot (cast `/Game/Characters/CharactersBlueprints/BP_NanoBot` OtherActor)
            (:`then`
              (`self.K2_DestroyActor` _asbp_nano_bot))
            (:`CastFailed`
              _))
          (`self.K2_DestroyActor`))))))

(fn `UserConstructionScript`)