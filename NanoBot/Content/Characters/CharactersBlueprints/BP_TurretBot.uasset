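; Turret bot, attached to a parent actor, that tracks and shoots at a BP_NanoBot entering its detection sphere.
; TargetPlayer re-calls itself through Delays, lerping rotation toward the bot with yaw clamped to an arc around the parent's yaw.
; Near alignment it spawns a BP_TurretProjectile and retargets after a second; out-of-arc targets are rechecked each second while valid.
; The second sphere's self-destruct is disconnected for easy difficulty.
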(event `SetUpTurret`
  (bind _rotationclampconstant (`self.RotationClampConstant`))
  (bind _yaw (.yaw (`self.K2_GetActorRotation` (`self.Parent`))))
  (`self.K2_AttachToActor` (`self.Parent`) "None" "KeepWorld" "KeepWorld" "KeepWorld")
  (set `self.MinRotation` (- _yaw _rotationclampconstant))
  (set `self.MaxRotation` (+ _yaw _rotationclampconstant)))

(event `self.ReceiveBeginPlay`)

(event `self.ReceiveTick`
  (params (DeltaSeconds :type "Float (single-precision)")))

(event `self.Sphere.OnComponentBeginOverlap`
  (params (OverlappedComponent :type "PrimitiveComponent Object Reference") (OtherActor :type "Actor Object Reference") (OtherComp :type "PrimitiveComponent Object Reference") (OtherBodyIndex :type Integer) (bFromSweep :type Boolean) (SweepResult :type "HitResult Structure (by ref)"))
  (bind _asbp_nano_bot (cast `/Game/Characters/CharactersBlueprints/BP_NanoBot` OtherActor))
  (set `self.Targetting` true)
  (set `self.BP_NanoBot` _asbp_nano_bot)
  (set `self.CurrentAlpha` 0.0)
  (`self.TargetPlayer` (`self.K2_GetActorRotation`) (`KismetMathLibrary.FindLookAtRotation` (`self.K2_GetActorLocation`) (`self.K2_GetActorLocation` (`self.BP_NanoBot`)))))

(event `self.Sphere.OnComponentEndOverlap`
  (params (OverlappedComponent :type "PrimitiveComponent Object Reference") (OtherActor :type "Actor Object Reference") (OtherComp :type "PrimitiveComponent Object Reference") (OtherBodyIndex :type Integer))
  (cast `/Game/Characters/CharactersBlueprints/BP_NanoBot` OtherActor)
  (set `self.Targetting` false)
  (set `self.BP_NanoBot` null))

(event `TargetPlayer`
  (params (StartRotation :type "Rotator Structure") (TargetRotation :type "Rotator Structure"))
  (bind _yaw (.yaw TargetRotation))
  (bind _rotationclampconstant (`self.RotationClampConstant`))
  (bind _rotationclampconstant_2 (`self.RotationClampConstant`))
  (bind _yaw_2 (.yaw (`self.K2_GetActorRotation` (`self.Parent`))))
  (bind _yaw_3 (.yaw (`self.K2_GetActorRotation` (`self.Parent`))))
  (bind _returnvalue (+ (`self.CurrentAlpha`) (* (`GameplayStatics.GetWorldDeltaSeconds`) (`self.RotationSpeed`))))
  (bind _returnvalue_2 (`KismetMathLibrary.RLerp` StartRotation TargetRotation _returnvalue true))
  (set `self.MinRotation` (- _yaw_3 _rotationclampconstant))
  (set `self.MaxRotation` (+ _yaw_3 _rotationclampconstant))
  (if (and (> _yaw (`self.MinRotation`)) (< _yaw (`self.MaxRotation`)))
    (`self.K2_SetActorRotation` (`KismetMathLibrary.MakeRotator` (.roll _returnvalue_2) (.pitch _returnvalue_2) (`KismetMathLibrary.FClamp` (.yaw _returnvalue_2) (`self.MinRotation`) (`self.MaxRotation`))))
    (set `self.CurrentAlpha` _returnvalue)
    (if (== _returnvalue_2 TargetRotation :`ErrorTolerance` 5.0)
      (set `self.MinRotation` (- _yaw_2 _rotationclampconstant_2))
      (set `self.MaxRotation` (+ _yaw_2 _rotationclampconstant_2))
      (`self.K2_SetActorRotation` (`KismetMathLibrary.MakeRotator` (.roll TargetRotation) (.pitch TargetRotation) (`KismetMathLibrary.FClamp` (.yaw TargetRotation) (`self.MinRotation`) (`self.MaxRotation`))))
      (`|SpawnActorFromClass` "/Game/Characters/CharactersBlueprints/BP_TurretProjectile.BP_TurretProjectile_C" (`KismetMathLibrary.MakeTransform` (+ (* (`SceneComponent.GetForwardVector` (`self.Arrow`)) 50.0) (`self.K2_GetActorLocation`)) (`self.K2_GetActorRotation`) (1.0 1.0 1.0)) "AdjustIfPossibleButAlwaysSpawn" "OverrideRootScale")
      (`KismetSystemLibrary.Delay` 1.0)
      (set `self.CurrentAlpha` 0.0)
      (`self.TargetPlayer` (`self.K2_GetActorRotation`) (`KismetMathLibrary.FindLookAtRotation` (`self.K2_GetActorLocation`) (`self.K2_GetActorLocation` (`self.BP_NanoBot`))))
      (else
        (`KismetSystemLibrary.Delay` 0.0)
        (`self.TargetPlayer` StartRotation TargetRotation)))
    (else
      (`KismetSystemLibrary.Delay` 1.0)
      (`/Engine/EditorBlueprintResources/StandardMacros.IsValid` (`self.BP_NanoBot`)
        (:`Is Valid`
          (`self.TargetPlayer` (`self.K2_GetActorRotation`) (`KismetMathLibrary.FindLookAtRotation` (`self.K2_GetActorLocation`) (`self.K2_GetActorLocation` (`self.BP_NanoBot`)))))))))

(event `self.Sphere1.OnComponentBeginOverlap`
  (params (OverlappedComponent :type "PrimitiveComponent Object Reference") (OtherActor :type "Actor Object Reference") (OtherComp :type "PrimitiveComponent Object Reference") (OtherBodyIndex :type Integer) (bFromSweep :type Boolean) (SweepResult :type "HitResult Structure (by ref)"))
  ;[1 1 1] Disconnect due to easy difficulty
)

(event `Key|R`
  (params (Key :type "Key Structure" :default "AnyKey"))
  (:`Pressed`
    (`KismetSystemLibrary.PrintString` (`KismetStringLibrary.Conv_DoubleToString` (`self.MinRotation`)))
    (`KismetSystemLibrary.PrintString` (`KismetStringLibrary.Conv_DoubleToString` (`self.MaxRotation`)))))

(fn `UserConstructionScript`)