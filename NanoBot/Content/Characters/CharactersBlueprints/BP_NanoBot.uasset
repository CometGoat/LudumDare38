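; BP_NanoBot is a bot launched slingshot-style by mouse drag that destroys any BP_BarrierBot its sphere hits.
; Releasing the mouse detaches it and feeds the drag vector through a timeline into ProjectileMovement velocity while turning it toward launch direction.
; Tick traces ahead to turn it onto approaching surface normals for landing.
; A recursive, delay-driven lerp handles rotation, finishing with a backward trace to align with the surface behind.
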(event `self.ReceiveBeginPlay`)

(event `CalculateVelocity`
  (params (StartVelocity :type "Vector Structure"))
  (bind (_direction _factor) (`Timeline|VelocityFactor` :!via `PlayFromStart`)
    (:`Update`
      (set `MovementComponent.Velocity` (* StartVelocity _factor) (`self.ProjectileMovement`)))))

(event `Key|LeftMouseButton`
  (params (Key :type "Key Structure" :default "AnyKey"))
  (bind (_locationx _locationy) (`PlayerController.GetMousePosition` (`GameplayStatics.GetPlayerController` 0)))
  (bind _returnvalue (- (`self.Vector_Start`) (`self.Vector_End`)))
  (bind _returnvalue_2 (`KismetMathLibrary.MakeVector` _locationx _locationy))
  (:`Pressed`
    (bind _output_get (set `self.Vector_Start` _returnvalue_2)))
  (:`Released`
    (set `self.Vector_End` _returnvalue_2)
    (`self.CalculateVelocity` _returnvalue)
    (`KismetSystemLibrary.PrintString` (`KismetStringLibrary.Conv_VectorToString` _returnvalue))
    (`self.K2_DetachFromActor` "KeepWorld" "KeepWorld" "KeepWorld")
    (set `self.IsAttached` false)
    (if (`self.Rotating`) :!label _label
      (`KismetSystemLibrary.Delay` 0.0)
      (goto _label)
      (else
        (set `self.CurrentRotationAlpha` 0.0)
        (`self.LerpRotation` (`self.K2_GetActorRotation`) (`KismetMathLibrary.Conv_VectorToRotator` _returnvalue))
        (set `self.Rotating` true)))))

(event `LerpRotation`
  (params (StartRotation :type "Rotator Structure") (TargetRotation :type "Rotator Structure"))
  (bind _returnvalue (`self.K2_GetActorRotation`))
  (bind _returnvalue_2 (`self.K2_GetActorLocation`))
  (bind _returnvalue_3 (+ (`self.CurrentRotationAlpha`) (* (`GameplayStatics.GetWorldDeltaSeconds`) 3.0)))
  (set `self.CurrentRotationAlpha` _returnvalue_3)
  (`self.K2_SetActorRotation` (`KismetMathLibrary.RLerp` StartRotation TargetRotation _returnvalue_3 true))
  (if (>= _returnvalue_3 1.0)
    (bind (_outhit _returnvalue_4) (`KismetSystemLibrary.LineTraceSingle` :`Start` _returnvalue_2 :`End` (+ _returnvalue_2 (* (`self.GetActorForwardVector`) -100.0)) :`TraceChannel` "TraceTypeQuery1" :`DrawDebugType` "ForOneFrame"))
    (if _returnvalue_4
      (bind _returnvalue_5 (`KismetMathLibrary.Conv_VectorToRotator` (`.ImpactNormal` (`GameplayStatics.BreakHitResult` _outhit))))
      (if (== _returnvalue_5 _returnvalue :`ErrorTolerance` 1.0)
        (`self.K2_SetActorRotation` _returnvalue_5)
        (set `self.Rotating` false)
        (else
          (`self.LerpRotation` _returnvalue _returnvalue_5)))
      (else
        (`self.K2_SetActorRotation` TargetRotation)
        (set `self.Rotating` false)))
    (else
      (`KismetSystemLibrary.Delay` 0.0)
      (`self.LerpRotation` StartRotation TargetRotation))))

(event `self.ReceiveTick`
  (params (DeltaSeconds :type "Float (single-precision)"))
  (bind _returnvalue (`self.K2_GetActorLocation`))
  (bind (_outhit _returnvalue_2) (`KismetSystemLibrary.LineTraceSingle` :`Start` _returnvalue :`End` (+ _returnvalue (* (`self.GetActorForwardVector`) 200.0)) :`TraceChannel` "TraceTypeQuery1" :`DrawDebugType` "ForOneFrame"))
  (if _returnvalue_2
    (bind _output_get (set `self.ImpactNormal` (`.ImpactNormal` (`GameplayStatics.BreakHitResult` _outhit))))
    (`self.RotateToLand` _output_get)))

(event `RotateToLand`
  (params (ImpactNormal :type "Vector Structure"))
  (if (`self.Rotating`) :!label _label_2
    (`KismetSystemLibrary.Delay` 0.0)
    (goto _label_2)
    (else
      (set `self.CurrentRotationAlpha` 0.0)
      (`self.LerpRotation` (`self.K2_GetActorRotation`) (`KismetMathLibrary.Conv_VectorToRotator` ImpactNormal))
      (set `self.Rotating` true))))

(event `self.Sphere.OnComponentBeginOverlap`
  (params (OverlappedComponent :type "PrimitiveComponent Object Reference") (OtherActor :type "Actor Object Reference") (OtherComp :type "PrimitiveComponent Object Reference") (OtherBodyIndex :type Integer) (bFromSweep :type Boolean) (SweepResult :type "HitResult Structure (by ref)")))

(event `self.Sphere.OnComponentHit`
  (params (HitComponent :type "PrimitiveComponent Object Reference") (OtherActor :type "Actor Object Reference") (OtherComp :type "PrimitiveComponent Object Reference") (NormalImpulse :type "Vector Structure") (Hit :type "HitResult Structure (by ref)"))
  (bind _asbp_barrier_bot (cast `/Game/Characters/CharactersBlueprints/BP_BarrierBot` OtherActor))
  (`self.K2_DestroyActor` _asbp_barrier_bot))

(event `Key|F`
  (params (Key :type "Key Structure" :default "AnyKey"))
  (:`Pressed`
    (`KismetSystemLibrary.PrintString` (`KismetStringLibrary.Conv_DoubleToString` (`ProjectileMovementComponent.Friction` (`self.ProjectileMovement`))))))

(event `CorrectLanding`
  (bind _returnvalue (`self.K2_GetActorLocation`))
  (bind (_outhit _returnvalue_2) (`KismetSystemLibrary.LineTraceSingle` :`Start` _returnvalue :`End` (+ _returnvalue (* (`self.GetActorForwardVector`) -100.0)) :`TraceChannel` "TraceTypeQuery1" :`DrawDebugType` "ForOneFrame"))
  (if _returnvalue_2
    (bind _output_get (set `self.ImpactNormal` (`.ImpactNormal` (`GameplayStatics.BreakHitResult` _outhit))))
    (`self.RotateToLand` _output_get)))

(event `Key|V`
  (params (Key :type "Key Structure" :default "AnyKey"))
  (:`Pressed`
    (`KismetSystemLibrary.PrintString` (`KismetStringLibrary.Conv_VectorToString` (`MovementComponent.Velocity` (`self.ProjectileMovement`))))))

(fn `UserConstructionScript`)