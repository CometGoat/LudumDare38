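; Master actor that builds concentric rotating wall rings on BeginPlay as BP_WallRing child actors spaced by RingDistance.
; Rings alternate spin direction via FlipFlop and slow with index by a power falloff; the innermost has turrets disabled.
; When SpawnBarrierBots is set, outer rings each get a counter-rotating BP_BarrierRing just inside, set up immediately.
; Finally, it runs SetUpWallRing on every BP_WallRing in the level.
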(event `self.ReceiveBeginPlay`
  (for _index (range 1 (+ (`self.RingNumber`) 1))
    (bind _returnvalue (`AddComponent|NODE_AddChildActorComponent-0` :`RelativeTransform` (`KismetMathLibrary.MakeTransform` (0.0 0.0 0.0))))
    (`ChildActorComponent.SetChildActorClass` _returnvalue "/Game/Environment/EnvironmentBlueprints/BP_WallRing.BP_WallRing_C")
    (bind _returnvalue_2 (== _index 1))
    (if _returnvalue_2
      (bind _asbp_wall_ring (cast `/Game/Environment/EnvironmentBlueprints/BP_WallRing` (`ChildActorComponent.ChildActor` _returnvalue) :!pure true))
      (set `/Game/Environment/EnvironmentBlueprints/BP_WallRing.SpawnTurrets` false _asbp_wall_ring))
    (bind _returnvalue_3 (* _index (`self.RingDistance`)))
    (set `/Game/Environment/EnvironmentBlueprints/BP_WallRing.WallDistance` _returnvalue_3 _asbp_wall_ring)
    (set `/Game/Environment/EnvironmentBlueprints/BP_WallRing.WallSpace` 3.0 _asbp_wall_ring)
    (`/Engine/EditorBlueprintResources/StandardMacros.FlipFlop`
      (:`A`
        (bind _returnvalue_4 (/ (`self.RingSpeed`) (`KismetMathLibrary.MultiplyMultiply_FloatFloat` (`KismetMathLibrary.Conv_IntToDouble` _index) 1.25)))
        (set `/Game/Environment/EnvironmentBlueprints/BP_WallRing.RotationSpeed` (`KismetMathLibrary.MakeRotator` 0.0 0.0 _returnvalue_4) _asbp_wall_ring))
      (:`B`
        (set `/Game/Environment/EnvironmentBlueprints/BP_WallRing.RotationSpeed` (`KismetMathLibrary.MakeRotator` 0.0 0.0 (* _returnvalue_4 -1.0)) _asbp_wall_ring)))
    (if (and (not _returnvalue_2) (`self.SpawnBarrierBots`))
      (`|ExecutionSequence`
        (:`then_0`
          (bind _returnvalue_5 (`AddComponent|NODE_AddChildActorComponent-1` :`RelativeTransform` (`KismetMathLibrary.MakeTransform` (0.0 0.0 0.0) (struct) (1.0 1.0 1.0))))
          (`ChildActorComponent.SetChildActorClass` _returnvalue_5 "/Game/Environment/EnvironmentBlueprints/BP_BarrierRing.BP_BarrierRing_C")
          (bind _asbp_barrier_ring (cast `/Game/Environment/EnvironmentBlueprints/BP_BarrierRing` (`ChildActorComponent.ChildActor` _returnvalue_5) :!pure true))
          (set `/Game/Environment/EnvironmentBlueprints/BP_BarrierRing.BotDistance` (- _returnvalue_3 500.0) _asbp_barrier_ring)
          (set `/Game/Environment/EnvironmentBlueprints/BP_BarrierRing.RotationSpeed` (* (`/Game/Environment/EnvironmentBlueprints/BP_WallRing.RotationSpeed` _asbp_wall_ring) -1.0) _asbp_barrier_ring)
          (set `/Game/Environment/EnvironmentBlueprints/BP_BarrierRing.BotSpace` (`self.BarrierBotSpace`) _asbp_barrier_ring)
          (`/Game/Environment/EnvironmentBlueprints/BP_BarrierRing.SetUpBarrierRing` _asbp_barrier_ring)))))
  (bind _outactors (`GameplayStatics.GetAllActorsOfClass` "/Game/Environment/EnvironmentBlueprints/BP_WallRing.BP_WallRing_C"))
  (for _array_element _outactors
    (`/Game/Environment/EnvironmentBlueprints/BP_WallRing.SetUpWallRing` _array_element)))

(fn `UserConstructionScript`)