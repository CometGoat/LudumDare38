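; BP_Planet is a planet actor that randomizes its look and viewing angle, then becomes the player's view.
; On BeginPlay it moves its camera to a random preset from PositionArray.
; It creates a dynamic M_Planet material on the sphere with random planet and atmosphere colours, keeping the atmosphere out of the darkest range.
; After a short delay, it sets itself as the player controller's view target.
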(event `self.ReceiveBeginPlay`
  (`SceneComponent.K2_SetRelativeLocation` (`self.Camera`) (`KismetArrayLibrary.Array_Get` (`self.PositionArray`) (`KismetMathLibrary.RandomInteger` 4)) false false)
  (bind _returnvalue (`PrimitiveComponent.CreateDynamicMaterialInstance` (`self.Sphere`) 0 "/Game/Environment/Materials/M_Planet.M_Planet"))
  (bind _output_get (set `self.DynamicMaterialReference` _returnvalue))
  (`MaterialInstanceDynamic.SetVectorParameterValue` _output_get "AtmosphereColour" (make `LinearColor` (`KismetMathLibrary.RandomFloatInRange` 0.25 1.0) (`KismetMathLibrary.RandomFloatInRange` 0.25 1.0) (`KismetMathLibrary.RandomFloatInRange` 0.25 1.0) 1.0))
  (`MaterialInstanceDynamic.SetVectorParameterValue` _output_get "PlanetColour" (make `LinearColor` (`KismetMathLibrary.RandomFloatInRange` 0.0 1.0) (`KismetMathLibrary.RandomFloatInRange` 0.0 1.0) (`KismetMathLibrary.RandomFloatInRange` 0.0 1.0) 1.0))
  (`KismetSystemLibrary.Delay` 0.2)
  (`PlayerController.SetViewTargetWithBlend` (`GameplayStatics.GetPlayerController` 0) self 0.0 "VTBlend_Linear" 0.0 false))

(fn `UserConstructionScript`)