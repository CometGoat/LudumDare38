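; BP_MazeWall is a maze wall actor that BP_NanoBot sticks to on impact.
; When its Cube is hit by a NanoBot, it reattaches the bot to itself keeping world transform, flags it attached, calls CorrectLanding and sets a nose cone material slot to neutral.
; Hits from a BP_Brick only print a debug message.
; A material loop and a landing sound are left unconnected.
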(event `self.Cube.OnComponentHit`
  (params (HitComponent :type "PrimitiveComponent Object Reference") (OtherActor :type "Actor Object Reference") (OtherComp :type "PrimitiveComponent Object Reference") (NormalImpulse :type "Vector Structure") (Hit :type "HitResult Structure (by ref)"))
  (bind _asbp_nano_bot (cast `/Game/Characters/CharactersBlueprints/BP_NanoBot` OtherActor)
    (:`then`
      (`self.K2_DetachFromActor` _asbp_nano_bot "KeepWorld" "KeepWorld" "KeepWorld")
      (`self.K2_AttachToActor` _asbp_nano_bot self "None" "KeepWorld" "KeepWorld" "KeepWorld" true)
      (set `/Game/Characters/CharactersBlueprints/BP_NanoBot.IsAttached` true _asbp_nano_bot)
      (`/Game/Characters/CharactersBlueprints/BP_NanoBot.CorrectLanding` _asbp_nano_bot)
      (`PrimitiveComponent.SetMaterial` (`/Game/Characters/CharactersBlueprints/BP_NanoBot.Cone` _asbp_nano_bot) 2 "/Game/Characters/Meshes/Player_NoseConeNeutral.Player_NoseConeNeutral"))
    (:`CastFailed`
      (cast `/Game/Environment/EnvironmentBlueprints/BP_Brick` OtherActor)
      (`KismetSystemLibrary.PrintString` "Attached player hit!"))))

(fn `UserConstructionScript`)