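; BP_BarrierRing is an actor that forms a rotating ring of BP_BarrierBot obstacles around its center.
; On BeginPlay it applies RotationSpeed to its RotatingMovement and derives the bot count from BotDistance, the ring radius, and BotSpace.
; It then adds child actor components evenly around the circle, each aimed at the center, and turns off each bot's own Moving flag.
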(event `self.ReceiveBeginPlay`
  (bind _returnvalue (`self.K2_GetActorLocation`))
  (bind _botnumber (`self.BotNumber`))
  (set `RotatingMovementComponent.RotationRate` (`self.RotationSpeed`) (`self.RotatingMovement`))
  (set `self.BotNumber` (`KismetMathLibrary.FTrunc` (/ (`self.BotDistance`) (* 17.78 (`self.BotSpace`)))))
  (for _index (range (+ _botnumber 1))
    (bind _returnvalue_2 (`KismetMathLibrary.RotateAngleAxis` (`KismetMathLibrary.MakeVector` (`self.BotDistance`)) (* _index (/ 360.0 (+ (`KismetMathLibrary.Conv_IntToDouble` _botnumber) 1.0))) (0.0 0.0 1.0)))
    (bind _returnvalue_3 (`AddComponent|NODE_AddChildActorComponent-0` :`RelativeTransform` (`KismetMathLibrary.MakeTransform` _returnvalue_2 (`KismetMathLibrary.FindLookAtRotation` (+ _returnvalue_2 _returnvalue) _returnvalue) (1.0 1.0 1.0))))
    (`ChildActorComponent.SetChildActorClass` _returnvalue_3 "/Game/Characters/CharactersBlueprints/BP_BarrierBot.BP_BarrierBot_C")
    (set `/Game/Characters/CharactersBlueprints/BP_BarrierBot.Moving` false (cast `/Game/Characters/CharactersBlueprints/BP_BarrierBot` (`ChildActorComponent.ChildActor` _returnvalue_3) :!pure true))))

(fn `UserConstructionScript`)