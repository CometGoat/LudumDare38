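; BP_Brick is a level brick whose BrickID decides how it reacts when a BP_NanoBot overlaps its box.
; Standard bricks attach the bot until it leaves, destructible bricks briefly make it bouncy then destroy themselves, and death bricks kill it.
; SetBrickID swaps in the destructible mesh, or gives standard bricks three BP_TurretBot child actors, either at random (unless NoTurrets) or via ForceTurrets.
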(event `SetBrickID`
  (bind _turretlocation (`self.TurretLocation`))
  (bind _relativelocation (`SceneComponent.RelativeLocation` _turretlocation))
  (switch `int` (`self.BrickID`)
    (:`0`
      (if (and (not (`self.NoTurrets`)) (== (`KismetMathLibrary.RandomIntegerInRange` 0 5) 0))
        (`|ExecutionSequence` :!label _label
          (:`then_0`
            (bind _returnvalue (`AddComponent|NODE_AddChildActorComponent-0` :`RelativeTransform` (`SceneComponent.GetRelativeTransform` _turretlocation)))
            (`ChildActorComponent.SetChildActorClass` _returnvalue "/Game/Characters/CharactersBlueprints/BP_TurretBot.BP_TurretBot_C")
            (bind _asbp_turret_bot (cast `/Game/Characters/CharactersBlueprints/BP_TurretBot` (`ChildActorComponent.ChildActor` _returnvalue) :!pure true))
            (set `/Game/Characters/CharactersBlueprints/BP_TurretBot.Parent` self _asbp_turret_bot)
            (`/Game/Characters/CharactersBlueprints/BP_TurretBot.SetUpTurret` _asbp_turret_bot))
          (:`then_1`
            (bind _returnvalue_2 (`AddComponent|NODE_AddChildActorComponent-1` :`RelativeTransform` (`KismetMathLibrary.MakeTransform` (+ _relativelocation (0.0 100.0 0.0)))))
            (`ChildActorComponent.SetChildActorClass` _returnvalue_2 "/Game/Characters/CharactersBlueprints/BP_TurretBot.BP_TurretBot_C")
            (bind _asbp_turret_bot_2 (cast `/Game/Characters/CharactersBlueprints/BP_TurretBot` (`ChildActorComponent.ChildActor` _returnvalue_2) :!pure true))
            (set `/Game/Characters/CharactersBlueprints/BP_TurretBot.Parent` self _asbp_turret_bot_2)
            (`/Game/Characters/CharactersBlueprints/BP_TurretBot.SetUpTurret` _asbp_turret_bot_2))
          (:`then_2`
            (bind _returnvalue_3 (`AddComponent|NODE_AddChildActorComponent-2` :`RelativeTransform` (`KismetMathLibrary.MakeTransform` (+ _relativelocation (0.0 -100.0 0.0)))))
            (`ChildActorComponent.SetChildActorClass` _returnvalue_3 "/Game/Characters/CharactersBlueprints/BP_TurretBot.BP_TurretBot_C")
            (bind _asbp_turret_bot_3 (cast `/Game/Characters/CharactersBlueprints/BP_TurretBot` (`ChildActorComponent.ChildActor` _returnvalue_3) :!pure true))
            (set `/Game/Characters/CharactersBlueprints/BP_TurretBot.Parent` self _asbp_turret_bot_3)
            (`/Game/Characters/CharactersBlueprints/BP_TurretBot.SetUpTurret` _asbp_turret_bot_3)))
        (elif (`self.ForceTurrets`)
          (goto _label))))
    (:`1`
      (`StaticMeshComponent.SetStaticMesh` (`self.Cube`) "/Game/Characters/Meshes/SM_Brick_Destructable.SM_Brick_Destructable"))))

(event `self.ReceiveBeginPlay`)

(event `self.Box.OnComponentHit`
  (params (HitComponent :type "PrimitiveComponent Object Reference") (OtherActor :type "Actor Object Reference") (OtherComp :type "PrimitiveComponent Object Reference") (NormalImpulse :type "Vector Structure") (Hit :type "HitResult Structure (by ref)")))

(event `self.Box.OnComponentBeginOverlap`
  (params (OverlappedComponent :type "PrimitiveComponent Object Reference") (OtherActor :type "Actor Object Reference") (OtherComp :type "PrimitiveComponent Object Reference") (OtherBodyIndex :type Integer) (bFromSweep :type Boolean) (SweepResult :type "HitResult Structure (by ref)"))
  (bind _asbp_nano_bot (cast `/Game/Characters/CharactersBlueprints/BP_NanoBot` OtherActor))
  (switch `int` (`self.BrickID`)
    (:`0`
      (if (not (`/Game/Characters/CharactersBlueprints/BP_NanoBot.IsAttached` _asbp_nano_bot))
        (`self.K2_AttachToActor` _asbp_nano_bot self "None" "KeepWorld" "KeepWorld" "KeepWorld" true)
        (set `/Game/Characters/CharactersBlueprints/BP_NanoBot.IsAttached` true _asbp_nano_bot)
        (`/Game/Characters/CharactersBlueprints/BP_NanoBot.CorrectLanding` _asbp_nano_bot)
        (`PrimitiveComponent.SetMaterial` (`/Game/Characters/CharactersBlueprints/BP_NanoBot.Cone` _asbp_nano_bot) 2 "/Game/Characters/Meshes/Player_NoseConeNeutral.Player_NoseConeNeutral")))
    (:`1`
      (`/Game/Characters/CharactersBlueprints/BP_NanoBot.StopBoostVelocity` _asbp_nano_bot)
      (bind _projectilemovement (`/Game/Characters/CharactersBlueprints/BP_NanoBot.ProjectileMovement` _asbp_nano_bot))
      (set `ProjectileMovementComponent.Bounciness` 1.0 _projectilemovement)
      (set `ProjectileMovementComponent.Friction` 0.0 _projectilemovement)
      (`KismetSystemLibrary.Delay` (`GameplayStatics.GetWorldDeltaSeconds`))
      (set `ProjectileMovementComponent.Bounciness` 0.0 _projectilemovement)
      (set `ProjectileMovementComponent.Friction` 1.0 _projectilemovement)
      (`self.K2_DestroyActor`))
    (:`2`
      (`/Game/Characters/CharactersBlueprints/BP_NanoBot.PlayerDeath` _asbp_nano_bot))))

(event `self.Box.OnComponentEndOverlap`
  (params (OverlappedComponent :type "PrimitiveComponent Object Reference") (OtherActor :type "Actor Object Reference") (OtherComp :type "PrimitiveComponent Object Reference") (OtherBodyIndex :type Integer))
  (bind _asbp_nano_bot (cast `/Game/Characters/CharactersBlueprints/BP_NanoBot` OtherActor))
  (if (and (`/Game/Characters/CharactersBlueprints/BP_NanoBot.IsAttached` _asbp_nano_bot) (== (`ActorComponent.GetOwner` (`SceneComponent.GetAttachParent` (`self.K2_GetRootComponent` OtherActor))) self))
    (`self.K2_DetachFromActor` _asbp_nano_bot "KeepWorld" "KeepWorld" "KeepWorld")
    (set `/Game/Characters/CharactersBlueprints/BP_NanoBot.IsAttached` false _asbp_nano_bot)))

(fn `BouncePlayer`
  (params (Player :type "/Game/Characters/CharactersBlueprints/BP_NanoBot Object Reference"))
  (set `ProjectileMovementComponent.Bounciness` 1.0 (`/Game/Characters/CharactersBlueprints/BP_NanoBot.ProjectileMovement` Player)))

(fn `UserConstructionScript`)