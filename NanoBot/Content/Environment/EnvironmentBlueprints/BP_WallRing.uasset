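; BP_WallRing is an actor that builds a rotating ring of BP_Brick walls around itself at BeginPlay.
; The brick count derives from WallDistance and WallSpace, and each brick is a child actor spaced evenly by angle and turned toward the center.
; Spawned bricks get BrickID 0, while a branch for ID 1 bricks is left unconnected.
; RotationSpeed drives the ring's spin through RotatingMovement.
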(event `self.ReceiveBeginPlay`
  (bind _returnvalue (`self.K2_GetActorLocation`))
  (bind _wallnumber (`self.WallNumber`))
  (set `RotatingMovementComponent.RotationRate` (`self.RotationSpeed`) (`self.RotatingMovement`))
  (set `self.WallNumber` (`KismetMathLibrary.FTrunc` (/ (`self.WallDistance`) (* 17.78 (`self.WallSpace`)))))
  (for _index (range (+ _wallnumber 1))
    (`/Engine/EditorBlueprintResources/StandardMacros.FlipFlop`
      (:`A`
        _)
      (:`B`
        _))
    (bind _returnvalue_2 (`KismetMathLibrary.RotateAngleAxis` (`KismetMathLibrary.MakeVector` (`self.WallDistance`)) (* _index (/ 360.0 (+ (`KismetMathLibrary.Conv_IntToDouble` _wallnumber) 1.0))) (0.0 0.0 1.0)))
    (bind _returnvalue_3 (`AddComponent|NODE_AddChildActorComponent-0` :`RelativeTransform` (`KismetMathLibrary.MakeTransform` _returnvalue_2 (`KismetMathLibrary.FindLookAtRotation` (+ _returnvalue_2 _returnvalue) _returnvalue) (1.0 1.0 1.0))))
    (`ChildActorComponent.SetChildActorClass` _returnvalue_3 "/Game/Environment/EnvironmentBlueprints/BP_Brick.BP_Brick_C")
    (bind _asbp_brick (cast `/Game/Environment/EnvironmentBlueprints/BP_Brick` (`ChildActorComponent.ChildActor` _returnvalue_3) :!pure true))
    (set `/Game/Environment/EnvironmentBlueprints/BP_Brick.BrickID` 0 _asbp_brick)
    (`/Game/Environment/EnvironmentBlueprints/BP_Brick.SetBrickID` _asbp_brick)))

(fn `UserConstructionScript`)